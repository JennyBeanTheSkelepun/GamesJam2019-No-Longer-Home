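; Behavior tree task that sends the pawn of a SisterController toward the actor stored in the Target blackboard key.
; On execute it casts and caches the owning controller, then calls AIMoveTo with the target actor, its location and a small acceptance radius.
; A successful move finishes the task as failed.
; A failed move or failed cast never calls FinishExecute.
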(event `self.ReceiveExecute`
  (params (OwnerActor :type "Actor Object Reference"))
  (bind _returnvalue (`BTFunctionLibrary.GetBlackboardValueAsActor` (`self.Target`)))
  (if (not (!= (`self.SisterController`) null))
    (bind _assister_controller (cast `/Game/Blueprints/AI/SisterController` OwnerActor))
    (set `self.SisterController` _assister_controller))
  (`|AIMoveTo` (`Controller.K2_GetPawn` (`self.SisterController`)) (`Actor.K2_GetActorLocation` _returnvalue) _returnvalue 50.0
    (:`OnSuccess`
      (`self.FinishExecute` false))))