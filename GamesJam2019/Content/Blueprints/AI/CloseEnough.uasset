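; CloseEnough is an AI condition check, apparently a Behavior Tree decorator, that tests the sister AI's distance to its target.
; It casts the owner to SisterController, stores it, and measures the distance from the controlled pawn to the Target blackboard actor.
; Despite the name, it passes when that distance is at least AcceptableDistance, meaning the pawn is at or beyond the threshold.
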(fn `PerformConditionCheck`
  (params (OwnerActor :type "Actor Object Reference"))
  (returns (ReturnValue :type Boolean))
  (bind _assister_controller (cast `/Game/Blueprints/AI/SisterController` OwnerActor))
  (set `self.SisterController` _assister_controller)
  (return (>= (`KismetMathLibrary.VSize` (- (`Actor.K2_GetActorLocation` (`BTFunctionLibrary.GetBlackboardValueAsActor` (`self.Target`))) (`Actor.K2_GetActorLocation` (`Controller.K2_GetPawn` (`self.SisterController`))))) (`self.AcceptableDistance`))))